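; Actor component that shows a drop shadow decal beneath its owning Character while it is not moving on the ground.
; BeginPlay caches the Character and spawns the decal attached to its mesh.
; Each tick updates visibility and, while airborne, line traces down the character's up axis to place the decal at the hit point.
; The decal shrinks as distance to the floor grows, using a clamped, inverted remap to drive a scale lerp.
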(event EventBeginPlay
  ;[0.4491 0.8591 1] Init Decal
  ;;[0.4491 0.8591 1] Cache player ref
  (bind _ascharacter (Utilities|Casting|CastToCharacter (Components|GetOwner)))
  (bind _output_get (Variables|Default|SetAs%20Character _ascharacter))
  ;;[0.4491 0.8591 1] Spawn decal and cache ref
  (bind _returnvalue (Class|GameplayStatics|SpawnDecalAttached "/Game/GPP/Materials/M_DecalDropShadow.M_DecalDropShadow" "5.000000,60.000000,60.000000" (Variables|/Script/Engine.Character|GetMesh _output_get) "None" "0, 0, 0" "90.000000,0.000000,0.000000" "KeepRelativeOffset" 0.0))
  (Variables|Default|SetDropDecal _returnvalue))

(event EventTick
  (params (DeltaSeconds :type Float%20%28single-precision%29))
  (bind _returnvalue (CallFunction|ShouldShowDecal))
  (bind _dropdecal (Variables|Default|GetDropDecal))
  (bind _as_character (Variables|Default|GetAs%20Character))
  (bind _returnvalue_2 (Transformation|GetActorLocation _as_character))
  ;[0.4491 0.8591 1] Update Drop Shadow
  ;;[0.4491 0.8591 1] Update visibility
  (Rendering|SetVisibility (Variables|Default|GetDropDecal) _returnvalue false)
  (if _returnvalue
    ;;[0.4491 0.8591 1] Check where the ground is underneath the player
    (bind _outhit (Class|KismetSystemLibrary|LineTraceSinglebyProfile _returnvalue_2 (- _returnvalue_2 (* (Transformation|GetActorUpVector _as_character) 1e+04)) "BlockAll" false (Utilities|Array|MakeArray _as_character) "None" true))
    (Utilities|FlowControl|Sequence
      (:then_0
        ;;[0.4491 0.8591 1] Set decal location to that point
        (Transformation|SetWorldLocation _dropdecal (.location _outhit) false false))
      (:then_1
        ;;[0.4491 0.8591 1] Scale decal based on distance to floor
        (Transformation|SetRelativeScale3D _dropdecal (Math|Vector|Lerp(Vector) "0.250000,0.250000,0.250000" "1.000000,1.000000,1.000000" (- 1.0 (Math|Float|MapRangeClamped (.distance _outhit) 0.0 2e+02 0.0 1.0))))))))

(fn ShouldShowDecal
  (return (not (AI|Components|NavMovement|IsMovingonGround (Variables|/Script/Engine.Character|GetCharacterMovement (Variables|Default|GetAs%20Character))))))