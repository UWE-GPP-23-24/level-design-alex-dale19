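; Checkpoint manager that tracks the player's last reached checkpoint and respawns the player there on death.
; On BeginPlay it marks the first checkpoint in its array as current and reached, then binds to the player's death and every checkpoint's reached event.
; Reached events update the current checkpoint, deaths respawn the player at its volume, and all bindings are removed on Destroyed.
; Helper functions return the initial checkpoint or look one up by bounds-checked ID.
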(event Custom|UpdateCheckpointReached
  (params (CheckpointReached :type BP%20Checkpoint%20Object%20Reference))
  ;[0.4491 0.8591 1] Handle checkpoint bindings
  (Variables|Default|SetCurrentCheckpoint CheckpointReached))

(event Custom|RespawnPlayer
  ;[0.4491 0.8591 1] Bind and Unbind player death
  ;;[0.4491 0.8591 1] Respawn Player
  (Default|Respawn (Variables|Default|GetAs%20BP%20Player%20Character) (Transformation|GetWorldLocation (Variables|/Game/GPP/Blueprints/Checkpoint_System/BP_Checkpoint.BP_Checkpoint_C|GetVolume (Variables|Default|GetCurrentCheckpoint)))))

(event EventBeginPlay
  ;[0.4491 0.8591 1] Init first checkpoint
  (bind _output_get (Variables|Default|SetInitialCheckpoint (Utilities|Array|Get(acopy) (Variables|Default|GetCheckpoints))))
  (bind _output_get_2 (Variables|Default|SetCurrentCheckpoint _output_get))
  (Default|UpdateMeshColour _output_get_2 (Variables|/Game/GPP/Blueprints/Checkpoint_System/BP_Checkpoint.BP_Checkpoint_C|GetReachedColour _output_get_2))
  ;[0.4491 0.8591 1] Bind and Unbind player death
  (bind _asbp_player_character (Utilities|Casting|CastToBP_PlayerCharacter (Game|GetPlayerCharacter 0)))
  (bind _output_get_3 (Variables|Default|SetAs%20BP%20Player%20Character _asbp_player_character))
  (EventDispatchers|BindEventtoOnPlayerDied _output_get_3 (delegate Custom|RespawnPlayer))
  ;[0.4491 0.8591 1] Handle checkpoint bindings
  ;;[0.4491 0.8591 1] Bind to each checkpoints OnReachedCheckpoint
  (for _array_element (Variables|Default|GetCheckpoints)
    (EventDispatchers|BindEventtoOnReachedCheckpoint _array_element (delegate Custom|UpdateCheckpointReached))))

(event EventDestroyed
  ;[0.4491 0.8591 1] Bind and Unbind player death
  (EventDispatchers|UnbindEventfromOnPlayerDied (Variables|Default|GetAs%20BP%20Player%20Character) (delegate Custom|RespawnPlayer))
  ;[0.4491 0.8591 1] Handle checkpoint bindings
  ;;[0.4491 0.8591 1] Clean up bindings
  (for _array_element (Variables|Default|GetCheckpoints)
    (EventDispatchers|UnbindEventfromOnReachedCheckpoint _array_element (delegate Custom|UpdateCheckpointReached))))

(fn ConstructionScript)

(fn GetInitialCheckpoint
  ;[0.4491 0.8591 1] Get first checkpoint in array
  (return (Utilities|Array|Get(acopy) (Variables|Default|GetCheckpoints))))

(fn GetCheckpointfromID
  (params (CheckpointID :type Integer))
  ;[0.4491 0.8591 1] If invalid return null, otherwise return checkpoint
  (if (or (< CheckpointID 0) (>= CheckpointID (Utilities|Array|Length (Variables|Default|GetCheckpoints))))
    (return 0)
    (else
      (return (Utilities|Array|Get(acopy) (Variables|Default|GetCheckpoints) CheckpointID)))))