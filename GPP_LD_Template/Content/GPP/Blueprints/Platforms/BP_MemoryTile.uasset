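; Memory puzzle floor tile that reacts when the player steps on it, according to its IsSafe flag.
; Box overlap plays a sound and tints the tile's dynamic material green if safe, red if not, with a FadeOut timeline driving FadeStrength.
; Unsafe tiles also teleport the player after a short delay to the TargetPoint returned by GetActorOfClass.
; The material instance is created in both the Construction Script and BeginPlay.
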(event OnComponentBeginOverlap(Box)
  (params (OverlappedComponent :type Primitive%20Component%20Object%20Reference) (OtherActor :type Actor%20Object%20Reference) (OtherComp :type Primitive%20Component%20Object%20Reference) (OtherBodyIndex :type Integer) (bFromSweep :type Boolean) (SweepResult :type Hit%20Result%20Structure%20%28by%20ref%29))
  (bind _dynamictilemat (Variables|Default|GetDynamicTileMat))
  (bind _asbp_player_character (Utilities|Casting|CastToBP_PlayerCharacter OtherActor))
  (if (Variables|Default|GetIsSafe)
    (Audio|SpawnSoundatLocation 0 (Transformation|GetWorldLocation (Variables|Default|GetBox)) "0, 0, 0" 1.0 1.0 0.0 "/Game/GPP/Blueprints/Components/NewSoundAttenuation.NewSoundAttenuation" 0)
    (Rendering|Material|SetVectorParameterValue _dynamictilemat "TintColor" "(R=0.420773,G=1.000000,B=0.495052,A=1.000000)" :!class /Script/Engine.MaterialInstanceDynamic)
    (bind _fadeout (Timeline|FadeOut PlayFromStart)
      (:Update
        (Rendering|Material|SetScalarParameterValue _dynamictilemat "FadeStrength" _fadeout :!class /Script/Engine.MaterialInstanceDynamic)))
    (else
      (bind _returnvalue (Actor|GetActorOfClass "/Script/Engine.TargetPoint"))
      (Audio|SpawnSoundatLocation "/Game/GPP/Blueprints/Components/wrong.wrong" (Transformation|GetWorldLocation (Variables|Default|GetBox)) "0, 0, 0" 1.0 1.0 0.0 0 0)
      (Rendering|Material|SetVectorParameterValue (Variables|Default|GetDynamicTileMat) "TintColor" "(R=1.000000,G=0.218681,B=0.228628,A=1.000000)" :!class /Script/Engine.MaterialInstanceDynamic)
      (Utilities|FlowControl|Sequence
        (:then_0
          (Timeline|FadeOut PlayFromStart))
        (:then_1
          (Utilities|FlowControl|Delay 0.2)
          (Transformation|Teleport _asbp_player_character (Transformation|GetActorLocation _returnvalue) "0, 0, 0"))))))

(event EventBeginPlay
  (bind _returnvalue (Rendering|Material|CreateDynamicMaterialInstance (Variables|Default|GetCube) 0 "/Game/StarterContent/Materials/TileTexutre.TileTexutre" "None" :!class /Script/Engine.PrimitiveComponent))
  (bind _output_get (Variables|Default|SetDynamicTileMat _returnvalue))
  (Rendering|Material|SetMaterial (Variables|Default|GetCube) 0 _output_get))

(event Collision|EventActorBeginOverlap
  (params (OtherActor :type Actor%20Object%20Reference)))

(event EventTick
  (params (DeltaSeconds :type Float%20%28single-precision%29)))

(fn ConstructionScript
  (bind _returnvalue (Rendering|Material|CreateDynamicMaterialInstance (Variables|Default|GetCube) 0 "/Game/StarterContent/Materials/TileTexutre.TileTexutre" "None" :!class /Script/Engine.PrimitiveComponent))
  (bind _output_get (Variables|Default|SetDynamicTileMat _returnvalue))
  (Rendering|Material|SetMaterial (Variables|Default|GetCube) 0 _output_get))