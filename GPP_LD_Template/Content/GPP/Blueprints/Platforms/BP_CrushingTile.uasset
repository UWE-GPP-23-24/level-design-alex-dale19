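; A crushing platform tile that moves as a floor or ceiling piece and can kill the player.
; Construction randomizes whether it is safe, its snapped start delay and its travel distance.
; Unsafe tiles start a timeline on BeginPlay that lerps the cube up, or down for ceilings; ResetTile restarts it.
; Box overlap kills the player when Floor and Ceiling tags show them caught between opposing tiles.
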(event OnComponentBeginOverlap(Box)
  (params (OverlappedComponent :type Primitive%20Component%20Object%20Reference) (OtherActor :type Actor%20Object%20Reference) (OtherComp :type Primitive%20Component%20Object%20Reference) (OtherBodyIndex :type Integer) (bFromSweep :type Boolean) (SweepResult :type Hit%20Result%20Structure%20%28by%20ref%29))
  (bind _asbp_player_character (Utilities|Casting|CastToBP_PlayerCharacter OtherActor))
  (for _array_element (Collision|GetOverlappingActors _asbp_player_character "BP_CrushingTile_C" :!class /Script/Engine.Actor)
    (if (Actor|ActorHasTag self "Floor")
      (if (Actor|ActorHasTag _array_element "Ceiling")
        (Default|KillPlayer _asbp_player_character :!label _label))
      (elif (Actor|ActorHasTag _array_element "Floor")
        (goto _label)))))

(event Custom|ActivateTile
  (if (not (Variables|Default|GetIsSafeTile))
    (Utilities|FlowControl|Delay (Variables|Default|GetInitialDelay))
    (bind _alpha (Timeline|CrushCycle PlayFromStart)
      (:Update
        (Transformation|SetRelativeLocation (Variables|Default|GetCube) (Math|Vector|Lerp(Vector) "0, 0, 0" (select (Variables|Default|GetIsCeilingTile) (Math|Vector|MakeVector 0.0 0.0 (* (Variables|Default|GetMoveDistance) -1.0)) (Math|Vector|MakeVector 0.0 0.0 (Variables|Default|GetMoveDistance))) _alpha) false false)))))

(event Custom|ResetTile
  (Utilities|FlowControl|Sequence
    (:then_0
      (bind _alpha (Timeline|CrushCycle Stop)
        (:Update
          (Transformation|SetRelativeLocation (Variables|Default|GetCube) (Math|Vector|Lerp(Vector) "0, 0, 0" (select (Variables|Default|GetIsCeilingTile) (Math|Vector|MakeVector 0.0 0.0 (* (Variables|Default|GetMoveDistance) -1.0)) (Math|Vector|MakeVector 0.0 0.0 (Variables|Default|GetMoveDistance))) _alpha) false false))))
    (:then_1
      (Transformation|SetRelativeLocation (Variables|Default|GetCube) "0, 0, 0" false false)
      (CallFunction|ActivateTile))))

(event EventBeginPlay
  (CallFunction|ActivateTile))

(event Collision|EventActorBeginOverlap
  (params (OtherActor :type Actor%20Object%20Reference)))

(event EventTick
  (params (DeltaSeconds :type Float%20%28single-precision%29)))

(fn ConstructionScript
  (Variables|Default|SetIsSafeTile (Math|Random|RandomBoolwithWeight (Variables|Default|GetsafeChance)))
  (Variables|Default|SetInitialDelay (Math|Float|SnapToGrid(Float) (Math|Random|RandomFloatinRange (Variables|Default|GetMinDelay) (Variables|Default|GetMaxDelay)) 0.5))
  (Variables|Default|SetMoveDistance (Math|Random|RandomFloatinRange (Variables|Default|GetMinDist) (Variables|Default|GetMaxDist))))