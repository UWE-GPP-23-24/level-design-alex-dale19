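; BP_QuickSliding is a platform Blueprint whose cube quickly slides to a target position when its trigger box is overlapped.
; BeginPlay caches the cube's relative location, and a DoOnce lets only the first overlap, by any actor, start the short MoveComponentTo toward EndLocation.
; The ResetDoors event moves the cube back to its cached start and re-arms the DoOnce so it can trigger again.
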(event OnComponentBeginOverlap(Box)
  (params (OverlappedComponent :type Primitive%20Component%20Object%20Reference) (OtherActor :type Actor%20Object%20Reference) (OtherComp :type Primitive%20Component%20Object%20Reference) (OtherBodyIndex :type Integer) (bFromSweep :type Boolean) (SweepResult :type Hit%20Result%20Structure%20%28by%20ref%29))
  (Utilities|FlowControl|DoOnce false
    (:Completed
      (Components|MoveComponentTo (Variables|Default|GetCube) (Variables|Default|GetEndLocation) "0, 0, 0" false false 0.3 false))))

(event Custom|ResetDoors
  (bind _cube (Variables|Default|GetCube))
  (Components|MoveComponentTo _cube (Variables|Default|GetStartLocation) "0, 0, 0" false false 0.2 false)
  (Utilities|FlowControl|DoOnce false) ; enters at Reset
)

(event EventBeginPlay
  (Variables|Default|SetStartLocation (Variables|/Script/Engine.SceneComponent|GetRelativeLocation (Variables|Default|GetCube))))

(event Collision|EventActorBeginOverlap
  (params (OtherActor :type Actor%20Object%20Reference)))

(event EventTick
  (params (DeltaSeconds :type Float%20%28single-precision%29)))

(fn ConstructionScript)